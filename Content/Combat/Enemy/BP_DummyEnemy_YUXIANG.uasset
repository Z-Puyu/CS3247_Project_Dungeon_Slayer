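; BP_DummyEnemy_YUXIANG is a simple test enemy for battles, where overlapping its Box tells FirstPersonGameMode to start a battle.
; ExecuteAction randomly picks one of two actions by coin flip: damage the stored Player, or raise a guard.
; TakeDamage spends an active guard to negate a hit and returns zero, otherwise it subtracts from Health and returns the remainder.
; IsAlive and EnemyDead provide the health check and actor destruction.
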(event OnComponentBeginOverlap(Box)
  (params (OverlappedComponent :type Primitive%20Component%20Object%20Reference) (OtherActor :type Actor%20Object%20Reference) (OtherComp :type Primitive%20Component%20Object%20Reference) (OtherBodyIndex :type Integer) (bFromSweep :type Boolean) (SweepResult :type Hit%20Result%20Structure%20%28by%20ref%29))
  (bind _asfirst_person_game_mode (Utilities|Casting|CastToFirstPersonGameMode (Game|GetGameMode)))
  (Default|StartBattle _asfirst_person_game_mode))

(event EventBeginPlay)

(event Collision|EventActorBeginOverlap
  (params (OtherActor :type Actor%20Object%20Reference)))

(event EventTick
  (params (DeltaSeconds :type Float%20%28single-precision%29)))

(event EventSetPlayer
  (params (Player :type BP%20FPS%20Object%20Reference))
  (Variables|Default|SetPlayer Player))

(fn ConstructionScript)

(fn RandomAction
  (Math|Float|CompareFloat (Math|Random|RandomFloat) 0.5
    (:>
      (Variables|Default|SetAction "NewEnumerator0" :!label _label))
    (:==
      (goto _label))
    (:<
      (Variables|Default|SetAction "NewEnumerator1"))))

(fn EnemyDead
  (Actor|DestroyActor)
  (return))

(fn ExecuteAction
  (CallFunction|RandomAction)
  (if (Utilities|Enum|Equal(Enum) (Variables|Default|GetAction) "NewEnumerator0")
    (Default|OnReceiveDamage (Variables|Default|GetPlayer) (Variables|Default|GetatkDamage))
    (else
      (Variables|Default|SetisGuard true)))
  (return (Utilities|String|EnumtoString (Variables|Default|GetAction))))

(fn IsAlive
  (Math|Integer|CompareInt (Variables|Default|GetHealth)
    (:>
      (return true))))

(fn TakeDamage
  (params (newHealth :type Integer))
  (if (Variables|Default|GetisGuard)
    (Variables|Default|SetisGuard false)
    (Development|PrintString (Utilities|String|EnumtoString (Variables|Default|GetAction)))
    (return 0)
    (else
      (bind _output_get (Variables|Default|SetHealth (- (Variables|Default|GetHealth) newHealth)))
      (return _output_get))))