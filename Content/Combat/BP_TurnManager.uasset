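; BP_TurnManager runs turn-based combat between the player and every BPI_Enemy actor in the level.
; On BeginPlay it creates the turn UI, gathers the enemies and starts the player's turn with a looping one-second countdown timer.
; A skip from the UI or an expired countdown triggers the enemy phase, where living enemies act and dead ones are removed.
; Turns repeat until no enemies remain, then it removes the UI and destroys itself.
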(event EventBeginPlay
  ;[0.15 0.15 0.15 0.5] Turn Initialization
  (bind _returnvalue (UserInterface|CreateWidget "/Game/Combat/WBP_TurnUI.WBP_TurnUI_C"))
  (bind _output_get (Variables|Default|SetturnUI _returnvalue))
  (UserInterface|Viewport|AddtoViewport _output_get 0)
  (Default|ToggleVisibility _output_get true)
  (bind _returnvalue_2 (Actor|GetActorOfClass "/Game/Combat/BP_Player.BP_Player_C"))
  (Variables|Default|Setplayer _returnvalue_2)
  (bind _outactors (Actor|GetAllActorswithInterface "/Game/Combat/Enemy/BPI_Enemy.BPI_Enemy_C"))
  (for _array_element _outactors
    (if (Utilities|DoesObjectImplementInterface _array_element "/Game/Combat/Enemy/BPI_Enemy.BPI_Enemy_C")
      (bind _asbpi_enemy (Utilities|Casting|CastToBPI_Enemy _array_element))
      (Utilities|Array|Add (Variables|Default|Getenemies) _asbpi_enemy)))
  (Variables|Default|SetplayerTurnEnds true)
  (CallFunction|OnPlayerTurnBegin))

(event Collision|EventActorBeginOverlap
  (params (OtherActor :type Actor%20Object%20Reference)))

(event EventTick
  (params (DeltaSeconds :type Float%20%28single-precision%29)))

(fn ConstructionScript)

(fn OnPlayerTurnEnd
  (bind _enemies (Variables|Default|Getenemies))
  (Development|PrintString "EnterLoop")
  (for _array_element _enemies
    (bind _alive (Default|IsAlive _array_element))
    (if _alive
      (bind _response (Default|ExecuteAction _array_element))
      (Development|PrintString _response)
      (else
        (Utilities|Array|RemoveItem (Variables|Default|Getenemies) _array_element)
        (Default|EnemyDead _array_element))))
  (Math|Integer|CompareInt (Utilities|Array|Length _enemies)
    (:>
      (CallFunction|OnPlayerTurnBegin))
    (:==
      (CallFunction|OnCombatEnd))))

(fn OnPlayerTurnBegin
  (bind _turn (Default|OnPlayerTurn (Variables|Default|Getplayer)))
  (Variables|Default|SetplayerTurnEnds _turn)
  (Variables|Default|Settimer 20)
  (bind _returnvalue (Utilities|Time|SetTimerbyFunctionName 0 "OnPlayerTurnTimer" 1.0 true))
  (Variables|Default|SettimeHandle _returnvalue))

(fn OnPlayerTurnTimer
  (bind _turnui (Variables|Default|GetturnUI))
  ;[0.15 0.15 0.15 0.5] Check if player turn ends
  (bind _newparam (Default|GetSkipped _turnui))
  (if _newparam
    (Default|UpdateTimerText _turnui)
    (Default|FalseSkipped _turnui)
    (else
      (Default|UpdateTimerText _turnui (Utilities|String|ToString(Integer) (Variables|Default|Gettimer)))
      (bind _result (Math|Integer|DecrementInt (Variables|Default|Gettimer))
        (:%20%20
          (bind _output_get (Variables|Default|Settimer _result))
          (Math|Integer|CompareInt _output_get
            (:==
              _)
            (:<
              _))))))
  (Utilities|Time|ClearandInvalidateTimerbyHandle (Variables|Default|GettimeHandle))
  (CallFunction|OnPlayerTurnEnd))

(fn OnCombatEnd
  (bind _turnui (Variables|Default|GetturnUI))
  (Default|ToggleVisibility _turnui false)
  (Widget|RemovefromParent _turnui)
  (Actor|DestroyActor))